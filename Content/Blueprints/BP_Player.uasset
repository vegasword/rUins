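; Player character with walk, run and jump controls, one-point damage and healing, a coin counter, and key-triggered respawn at its starting location.
; It creates the HUD on BeginPlay and offers mouse-wheel camera zoom.
; Tick drives a line-trace ground check that manages air control, plus an FOV blend while running.
; Tick also restarts a looping dirt VFX timer whenever not running on ground, so it fires only during sustained runs.
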(event OnSystemFinished(VFXEmitter)
  (params (PSystem :type Niagara%20Component%20Object%20Reference))
  ;[1 1 1] Updated states
  (Niagara|ReinitializeSystem PSystem))

(event EventTick
  (params (DeltaSeconds :type Float%20%28single-precision%29))
  ;[1 1 1] Updated states
  (Utilities|SetGroundedState)
  (Utilities|UpdateBackVFX)
  (Utilities|SetDynamicCameraFov DeltaSeconds))

(event EventBeginPlay
  ;[1 1 1] Create player HUD Instance
  (bind _returnvalue (UserInterface|CreateWidget "/Game/Blueprints/UI/BP_HUD.BP_HUD_C"))
  (Variables|/Game/Blueprints/UI/BP_HUD.BP_HUD_C|SetPlayerRef _returnvalue self)
  (UserInterface|Viewport|AddtoViewport _returnvalue 0))

(event Input|ActionEvents|InputActionJump
  (params (Key :type Key%20Structure :default "None"))
  ;[1 1 1] Movement inputs
  (:Pressed
    (Character|Jump)))

(event Input|ActionEvents|InputActionRun
  (params (Key :type Key%20Structure :default "None"))
  ;[1 1 1] Movement inputs
  (:Pressed
    (Utilities|SetRunState :!label _label))
  (:Released
    (goto _label Released)))

(event Input|ActionEvents|InputActionRespawn
  (params (Key :type Key%20Structure :default "None"))
  ;[1 1 1] Revive key (post death)
  (:Pressed
    (if (not (Variables|Default|GetIsAlive))
      (Transformation|SetActorLocation (Variables|Default|GetRespawnCoord) false true)
      (CallFunction|RevivePlayer))))

(event Input|AxisEvents|InputAxisForward
  (params (AxisValue :type Float%20%28single-precision%29))
  ;[1 1 1] Movement inputs
  (Pawn|Input|AddMovementInput (Math|Vector|GetForwardVector (Math|Rotator|MakeRotator 0.0 0.0 (.yaw (Pawn|GetControlRotation :!class /Script/Engine.Pawn)))) AxisValue false))

(event Input|AxisEvents|InputAxisLookup
  (params (AxisValue :type Float%20%28single-precision%29))
  ;[1 1 1] Mouse inputs
  (Pawn|Input|AddControllerPitchInput AxisValue))

(event Input|AxisEvents|InputAxisRight
  (params (AxisValue :type Float%20%28single-precision%29))
  ;[1 1 1] Movement inputs
  (Pawn|Input|AddMovementInput (Math|Vector|GetRightVector (Math|Rotator|MakeRotator 0.0 0.0 (.yaw (Pawn|GetControlRotation :!class /Script/Engine.Pawn)))) AxisValue false))

(event Input|AxisEvents|InputAxisLookRight
  (params (AxisValue :type Float%20%28single-precision%29))
  ;[1 1 1] Mouse inputs
  (Pawn|Input|AddControllerYawInput AxisValue))

(event Input|MouseEvents|MouseWheelAxis
  (params (AxisValue :type Float%20%28single-precision%29))
  ;[1 1 1] Mouse inputs
  (Utilities|SetSpringArmLength AxisValue))

(fn ConstructionScript
  (Variables|/Script/Engine.CharacterMovementComponent|SetMaxWalkSpeed (Variables|Character|GetCharacterMovement) (Variables|Default|GetWalkSpeed))
  (Variables|Default|SetHP (Variables|Default|GetMaxHP))
  (Variables|Default|SetZoom (Variables|/Script/Engine.SpringArmComponent|GetTargetArmLength (Variables|Default|GetSpringArm)))
  (Variables|Default|SetDefaultFOV (Variables|/Script/Engine.CameraComponent|GetFieldOfView (Variables|Default|GetCamera)))
  (Variables|Default|SetRespawnCoord (Transformation|GetActorLocation)))

(fn GainPoint
  (Math|Integer|IncrementInt (Variables|Default|GetCoins)))

(fn TakeDamage
  (if (<= (- (Variables|Default|GetHP) 1) 0)
    (Utilities|FlowControl|Sequence
      (:then_0
        (Math|Integer|DecrementInt (Variables|Default|GetHP) :!label _label))
      (:then_1
        (CallFunction|KillPlayer)))
    (else
      (goto _label))))

(fn Heal
  (if (and (<= (+ (Variables|Default|GetHP) 1) (Variables|Default|GetMaxHP)) (Variables|Default|GetIsAlive))
    (Math|Integer|IncrementInt (Variables|Default|GetHP)
      (:%20%20
        (return true)))
    (else
      (return false))))

(fn RevivePlayer
  (Variables|Default|SetIsAlive true)
  (Variables|Default|SetHP (Variables|Default|GetMaxHP))
  (Pawn|Components|CharacterMovement|SetMovementMode (Variables|Character|GetCharacterMovement) "MOVE_Walking" 0))

(fn KillPlayer
  (Variables|Default|SetIsAlive false)
  (Variables|Default|SetHP 0)
  (Pawn|Components|CharacterMovement|DisableMovement (Variables|Character|GetCharacterMovement)))

(fn SpawnCollectibleVFX
  (params (SystemTemplate :type Niagara%20System%20Object%20Reference))
  (Niagara|SpawnSystemAttached SystemTemplate (Variables|Default|GetVFX%20Emitter) "None" "0, 0, 0" "0, 0, 0" "KeepRelativeOffset" true true "AutoRelease"))

(fn SpawnBackVFX
  (Niagara|SpawnSystemAttached "/Game/External/SurfaceFootstepVFX/Niagara_FX/ParticleSystems/PSN_Dirt_Surface.PSN_Dirt_Surface" (Variables|Default|GetBack%20Emitter) "None" "0, 0, 0" "0, 0, 0" "KeepRelativeOffset" true true "AutoRelease"))