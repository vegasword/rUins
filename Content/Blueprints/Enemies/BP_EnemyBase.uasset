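; Base enemy that chases the player, hurts on contact and is defeated through hits on its weak point.
; Weak-point overlaps bounce the player and remove life, with a one-second cooldown; death may drop a heal pickup.
; Capsule hits knock the player back and deal repeating, delayed damage while overlap persists.
; A gated Tick check delegates chasing to BP_EnemyControler, which returns it to spawn when the player leaves detection range.
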(event OnComponentBeginOverlap(WeakPointCollider)
  (params (OverlappedComponent :type Primitive%20Component%20Object%20Reference) (OtherActor :type Actor%20Object%20Reference) (OtherComp :type Primitive%20Component%20Object%20Reference) (OtherBodyIndex :type Integer) (bFromSweep :type Boolean) (SweepResult :type Hit%20Result%20Structure%20%28by%20ref%29))
  ;[1 1 1] Enemy damaged
  (bind _asbp_player (Utilities|Casting|CastToBP_Player OtherActor))
  (Utilities|FlowControl|DoOnce false :!label _label
    (:Completed
      (bind _result (Math|Integer|DecrementInt (Variables|Default|GetLife))
        (:%20%20
          (Character|LaunchCharacter _asbp_player "0, 0,500.000000" false false)
          (if (<= _result 0)
            (Utilities|DropHeart)
            (Actor|DestroyActor)
            (else
              (Utilities|FlowControl|Delay 1.0)
              (goto _label Reset))))))))

(event OnComponentEndOverlap(DetectionRangeCollider)
  (params (OverlappedComponent :type Primitive%20Component%20Object%20Reference) (OtherActor :type Actor%20Object%20Reference) (OtherComp :type Primitive%20Component%20Object%20Reference) (OtherBodyIndex :type Integer))
  ;[1 1 1] AI Behavior related
  (Utilities|Casting|CastToBP_Player OtherActor)
  (CallFunction|GoBacktoSpawn false))

(event OnComponentHit(CapsuleComponent)
  (params (HitComponent :type Primitive%20Component%20Object%20Reference) (OtherActor :type Actor%20Object%20Reference) (OtherComp :type Primitive%20Component%20Object%20Reference) (NormalImpulse :type Vector :default "0, 0, 0") (Hit :type Hit%20Result%20Structure%20%28by%20ref%29))
  ;[1 1 1] Player damaged
  (bind _asbp_player (Utilities|Casting|CastToBP_Player OtherActor))
  (Character|LaunchCharacter _asbp_player (+ (* (.ImpactNormal (Collision|BreakHitResult Hit)) -8e+02) (Math|Vector|MakeVector 0.0 0.0 2.5e+02)) false false)
  (Utilities|InflictDamage _asbp_player))

(event Custom|Can%20Follow%20Player
  ;[1 1 1] AI Behavior related
  (Utilities|FollowPlayer?) ; enters at Open
)

(event Custom|Can't%20follow%20player
  ;[1 1 1] AI Behavior related
  (Utilities|FollowPlayer?) ; enters at Close
)

(event EventTick
  (params (DeltaSeconds :type Float%20%28single-precision%29))
  ;[1 1 1] AI Behavior related
  (Utilities|FollowPlayer?
    (:True
      (CallFunction|FollowPlayer))))

(fn ConstructionScript
  (Utilities|FlowControl|Sequence
    (:then_0
      (Variables|Default|SetLife (Variables|Default|GetMaxLife)))
    (:then_1
      (Components|Sphere|SetSphereRadius (Variables|Default|GetDetectionRangeCollider) (Variables|Default|GetDetectionRange) false))
    (:then_2
      (Variables|Default|SetSpawnPoint (Transformation|GetWorldLocation (Variables|Collision|GetCapsuleComponent))))))

(fn FollowPlayer
  (bind _asbp_enemy_controler (Utilities|Casting|CastToBP_EnemyControler (AI|GetAIController self)))
  (Default|FollowPlayer _asbp_enemy_controler))

(fn GoBacktoSpawn
  (params (For%20healing%20? :type Boolean))
  (bind _asbp_enemy_controler (Utilities|Casting|CastToBP_EnemyControler (AI|GetAIController self)))
  (Default|Goto _asbp_enemy_controler For%20healing%20? (Variables|Default|GetSpawnPoint)))