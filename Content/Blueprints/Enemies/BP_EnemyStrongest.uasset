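; BP_EnemyStrongest is an enemy variant with two max life and a weak point the player can hit.
; Overlapping the weak point with the player triggers, once, a stop in following and a return to spawn.
; The Heal event runs a delayed Regeneration that restores full life with a Niagara healing effect, then re-enables following and resets the one-shot gate.
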(event OnComponentBeginOverlap(WeakPointCollider)
  (params (OverlappedComponent :type Primitive%20Component%20Object%20Reference) (OtherActor :type Actor%20Object%20Reference) (OtherComp :type Primitive%20Component%20Object%20Reference) (OtherBodyIndex :type Integer) (bFromSweep :type Boolean) (SweepResult :type Hit%20Result%20Structure%20%28by%20ref%29))
  (Utilities|Casting|CastToBP_Player OtherActor)
  (Utilities|FlowControl|DoOnce false
    (:Completed
      (CallFunction|Can'tFollowPlayer)
      (CallFunction|GoBacktoSpawn true))))

(event Custom|Event%20Heal
  (Utilities|Regeneration)
  (CallFunction|CanFollowPlayer)
  (Utilities|FlowControl|DoOnce false) ; enters at Reset
)

(fn ConstructionScript
  (Variables|Default|SetMaxLife 2)
  (|CallParentFunction))