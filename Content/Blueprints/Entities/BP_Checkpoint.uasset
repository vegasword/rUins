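; BP_Checkpoint is a trigger volume that sets the player's respawn point.
; When a BP_Player overlaps its Box, the box's center of mass is written to that player's RespawnCoord.
; The construction script multiplies the box extent by its world scale.
; A separate KillPlayer function, not called in this graph, kills a living player through a DoOnce gate.
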(event OnComponentBeginOverlap(Box)
  (params (OverlappedComponent :type Primitive%20Component%20Object%20Reference) (OtherActor :type Actor%20Object%20Reference) (OtherComp :type Primitive%20Component%20Object%20Reference) (OtherBodyIndex :type Integer) (bFromSweep :type Boolean) (SweepResult :type Hit%20Result%20Structure%20%28by%20ref%29))
  (bind _asbp_player (Utilities|Casting|CastToBP_Player OtherActor))
  (Variables|/Game/Blueprints/BP_Player.BP_Player_C|SetRespawnCoord _asbp_player (Physics|GetCenterOfMass (Variables|Default|GetBox) "None")))

(fn ConstructionScript
  (bind _box (Variables|Default|GetBox))
  (Components|Box|SetBoxExtent _box (* (Variables|/Script/Engine.BoxComponent|GetBoxExtent _box) (Transformation|GetWorldScale _box)) true))